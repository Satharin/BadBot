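; BP_SphereSpawner periodically spawns BP_SmallSphere actors at random points within a spherical radius around itself.
; BeginPlay starts a looping timer on SpawnTime that spawns each sphere with a random rotation.
; Positions come from a random direction scaled by a random distance up to SpawnRadius, so spawns cluster toward the center.
; A debug sphere showing the spawn range exists but is disconnected.
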(event `self.ReceiveBeginPlay`
  ;[1 0.02901 0] Start Sphere Spawn Timer
  (`KismetSystemLibrary.K2_SetTimerDelegate` (delegate `SpawnSmallSphere`) (`self.SpawnTime`) true))

(event `SpawnSmallSphere`
  ;[1 0.02901 0] Start Sphere Spawn Timer
  (`|SpawnActorFromClass` "/Game/Blueprints/SmallSphere/BP_SmallSphere.BP_SmallSphere_C" (`KismetMathLibrary.MakeTransform` (`self.GetRandomPointInSphereRadius`) (`KismetMathLibrary.RandomRotator` false)) "Undefined" "MultiplyWithRoot" null null))

(event `self.ReceiveTick`
  (params (DeltaSeconds :type "Float (single-precision)")))

(fn `GetRandomPointInSphereRadius`
  (returns (RandomPoint :type "Vector Structure"))
  (return (+ (`self.K2_GetActorLocation`) (* (`KismetMathLibrary.GetForwardVector` (`KismetMathLibrary.RandomRotator` false)) (`KismetMathLibrary.RandomFloatInRange` 0.0 (`self.SpawnRadius`))))))

(fn `UserConstructionScript`)